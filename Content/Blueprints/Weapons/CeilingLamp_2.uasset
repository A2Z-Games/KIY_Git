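; CeilingLamp_2 is a ceiling lamp Blueprint in the weapons folder that attaches as a second weapon through its Attach2ndWeapon event.
; With HasWeapon true, it sphere-traces from its Sphere component, prints the hit component's name and snaps onto that component's "Socket".
; The trace end is the scaled forward vector alone, without the start location added.
; Interact and overlap events are empty; Chair-cast and player-hand attach logic is disconnected.
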(event OnComponentBeginOverlap(Sphere)
  (params (OverlappedComponent :type Primitive%20Component%20Object%20Reference) (OtherActor :type Actor%20Object%20Reference) (OtherComp :type Primitive%20Component%20Object%20Reference) (OtherBodyIndex :type Integer) (bFromSweep :type Boolean) (SweepResult :type Hit%20Result%20Structure%20%28by%20ref%29)))

(event EventAttach2ndWeapon
  (params (Has%20Weapon :type Boolean))
  (if Has%20Weapon
    (bind _outhit (Collision|SphereTraceByChannel (Transformation|GetWorldLocation (Variables|Default|GetSphere)) (* (Math|Vector|GetForwardVector (Transformation|GetActorRotation)) 5e+01) 4e+01 "TraceTypeQuery1" false 0 "Persistent"))
    (Development|PrintString (Utilities|GetDisplayName (.hitcomponent _outhit)))
    (Transformation|AttachComponentToComponent (.hitcomponent _outhit) "Socket" "SnapToTarget" "SnapToTarget" "SnapToTarget" false)
    (else
      (Development|PrintString "Hello"))))

(event EventInteract
  (params (Interacter :type Actor%20Object%20Reference) (HasWeapon :type Boolean)))

(fn ConstructionScript)