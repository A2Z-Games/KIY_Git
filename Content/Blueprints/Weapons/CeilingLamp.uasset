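; Ceiling lamp that responds to an Interact event by attaching itself as a weapon on the player or onto a Chair.
; Without a held weapon, it snaps to the first player character's mesh at the Weapon socket, keeping world rotation and scale.
; With a weapon held, it attaches to a Chair interacter's mesh socket using relative transforms, or prints a fallback message for other interacters.
; Both branches print the HasWeapon flag for debugging.
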(event EventInteract
  (params (Interacter :type Object%20Object%20Reference) (HasWeapon :type Boolean))
  (if HasWeapon
    (Development|PrintString (Utilities|String|ToString(Boolean) HasWeapon))
    (bind _aschair (Utilities|Casting|CastToChair Interacter)
      (:then
        (Transformation|AttachComponentToComponent (Variables|/Script/Engine.StaticMeshActor|GetStaticMeshComponent _aschair) "Socket" "KeepRelative" "KeepRelative" "KeepRelative" false))
      (:CastFailed
        (Development|PrintString "Hello")))
    (else
      (Development|PrintString (Utilities|String|ToString(Boolean) HasWeapon))
      (Transformation|AttachComponentToComponent (Variables|/Script/Engine.Character|GetMesh (Game|GetPlayerCharacter 0)) "Weapon" "SnapToTarget" "KeepWorld" "KeepWorld" false))))

(fn ConstructionScript)