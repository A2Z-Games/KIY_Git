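; FarkashWeapon is a melee weapon actor the player can pick up, drop and wear out until it breaks.
; PickUp snaps the mesh to the "Weapon" socket of the ThirdPersonCharacter cached at BeginPlay, and Drop detaches it in place.
; Each Break call lowers Durability, playing a sword-break sound and destroying the actor at zero.
; The Highlight volume toggles a custom-depth stencil outline, which Tick keeps off while held.
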(event OnComponentEndOverlap(Hit)
  (params (OverlappedComponent :type Primitive%20Component%20Object%20Reference) (OtherActor :type Actor%20Object%20Reference) (OtherComp :type Primitive%20Component%20Object%20Reference) (OtherBodyIndex :type Integer)))

(event OnComponentBeginOverlap(WeaponPlacement)
  (params (OverlappedComponent :type Primitive%20Component%20Object%20Reference) (OtherActor :type Actor%20Object%20Reference) (OtherComp :type Primitive%20Component%20Object%20Reference) (OtherBodyIndex :type Integer) (bFromSweep :type Boolean) (SweepResult :type Hit%20Result%20Structure%20%28by%20ref%29)))

(event OnComponentBeginOverlap(Highlight)
  (params (OverlappedComponent :type Primitive%20Component%20Object%20Reference) (OtherActor :type Actor%20Object%20Reference) (OtherComp :type Primitive%20Component%20Object%20Reference) (OtherBodyIndex :type Integer) (bFromSweep :type Boolean) (SweepResult :type Hit%20Result%20Structure%20%28by%20ref%29))
  (bind _staticmesh (Variables|Default|GetStaticMesh))
  (Rendering|SetRenderCustomDepth _staticmesh true)
  (Rendering|SetCustomDepthStencilValue _staticmesh 2))

(event OnComponentEndOverlap(Highlight)
  (params (OverlappedComponent :type Primitive%20Component%20Object%20Reference) (OtherActor :type Actor%20Object%20Reference) (OtherComp :type Primitive%20Component%20Object%20Reference) (OtherBodyIndex :type Integer))
  (bind _staticmesh (Variables|Default|GetStaticMesh))
  (Rendering|SetRenderCustomDepth _staticmesh false)
  (Rendering|SetCustomDepthStencilValue _staticmesh 0))

(event EventDrop
  (if (Variables|Default|GetHasWeapon)
    (Transformation|DetachFromComponent (Variables|Default|GetStaticMesh) "KeepWorld" "KeepRelative" "KeepWorld" true)
    (Variables|Default|SetHasWeapon false)
    (else
      (Development|PrintString "Nothing to drop"))))

(event EventPickUp
  (Transformation|AttachComponentToComponent (Variables|Default|GetStaticMesh) (Variables|/Script/Engine.Character|GetMesh (Variables|Default|GetPlayerRef)) "Weapon" "SnapToTarget" "SnapToTarget" "SnapToTarget" false)
  (Variables|Default|SetHasWeapon true))

(event EventBreak
  (Variables|Default|SetDurability (- (Variables|Default|GetDurability) 1e+01))
  (if (<= (Variables|Default|GetDurability) 0.0)
    (Audio|PlaySoundatLocation "/Game/KIY/DEV/Tomer/Sword_Break.Sword_Break" (Transformation|GetWorldLocation (Variables|Default|GetHit)) "0, 0, 0" 1.0 1.0 0.0 0 0 0)
    (Actor|DestroyActor)))

(event EventBeginPlay
  (bind _asthird_person_character (Utilities|Casting|CastToThirdPersonCharacter (Game|Player|GetPlayerPawn 0)))
  (Variables|Default|SetPlayerRef _asthird_person_character))

(event EventTick
  (params (DeltaSeconds :type Float%20%28single-precision%29))
  (bind _staticmesh (Variables|Default|GetStaticMesh))
  (if (Variables|Default|GetHasWeapon)
    (Rendering|SetRenderCustomDepth _staticmesh false)
    (Rendering|SetCustomDepthStencilValue _staticmesh 0)))

(fn ConstructionScript)