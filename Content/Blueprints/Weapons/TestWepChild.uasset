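; TestWepChild is a test child weapon Blueprint that can attach itself as a second weapon to its parent actor.
; Attach2ndWeapon prints the HasWeapon flag and, when true, snaps the actor to CubeSocket on the parent actor.
; Interact only prints a debug message, and an unconnected component-attach variant remains unused.
; The construction script just calls the parent's.
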(event EventAttach2ndWeapon
  (params (Has%20Weapon :type Boolean))
  (Development|PrintString (Utilities|String|ToString(Boolean) Has%20Weapon))
  (if Has%20Weapon
    (Transformation|AttachActorToActor (Actor|GetParentActor) "CubeSocket" "SnapToTarget" "SnapToTarget" "SnapToTarget" false)
    (else
      (Development|PrintString "false"))))

(event EventInteract
  (params (Interacter :type Actor%20Object%20Reference) (HasWeapon :type Boolean))
  (Development|PrintString "Nope"))

(fn ConstructionScript
  (|CallParentFunction))