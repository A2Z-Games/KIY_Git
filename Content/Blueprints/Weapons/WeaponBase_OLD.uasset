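; Legacy base Blueprint for weapon pickups that highlight on overlap and can be added to the player's inventory.
; The Highlight component's overlaps toggle custom depth and stencil on the static mesh, and Tick clears it once the weapon is stored.
; AddToInv passes a non-stackable slot struct with self references to InventoryComponentOLD, then destroys the actor on success.
; A separate Destroy event removes only the mesh to keep box collision.
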(event OnComponentEndOverlap(Highlight)
  (params (OverlappedComponent :type Primitive%20Component%20Object%20Reference) (OtherActor :type Actor%20Object%20Reference) (OtherComp :type Primitive%20Component%20Object%20Reference) (OtherBodyIndex :type Integer))
  (bind _staticmesh (Variables|Default|GetStaticMesh))
  ;[1 1 1] Highlight
  (Rendering|SetRenderCustomDepth _staticmesh false)
  (Rendering|SetCustomDepthStencilValue _staticmesh 0))

(event OnComponentBeginOverlap(Highlight)
  (params (OverlappedComponent :type Primitive%20Component%20Object%20Reference) (OtherActor :type Actor%20Object%20Reference) (OtherComp :type Primitive%20Component%20Object%20Reference) (OtherBodyIndex :type Integer) (bFromSweep :type Boolean) (SweepResult :type Hit%20Result%20Structure%20%28by%20ref%29))
  (bind _staticmesh (Variables|Default|GetStaticMesh))
  ;[1 1 1] Highlight
  (Rendering|SetRenderCustomDepth _staticmesh true)
  (Rendering|SetCustomDepthStencilValue _staticmesh 2))

(event Custom|Destroy
  ;[1 1 1] used in order to maintain BP Box collision
  (Components|DestroyComponent (Variables|Default|GetStaticMesh)))

(event Custom|AddToInv
  ;[1 1 1] Add To Inventory
  (bind _success (Default|AddtoInventory (Actor|GetComponentbyClass (Game|GetPlayerCharacter 0) "/Game/InventorySystem/InventoryComponentOLD.InventoryComponentOLD_C") (Utilities|Struct|MakeSlotStruct (Utilities|Struct|MakeItemStruct (Utilities|Text|ToText(String) (Utilities|GetObjectName self)) false (Variables|Default|GetWeaponDurability) "" (Variables|Default|GetThumbnail) false 1 0 0 self (Variables|Default|GetStaticMesh)) 1 self)))
  (Development|PrintString (Utilities|GetDisplayName (.weaponref (Variables|Default|GetItemStructure))))
  (if _success
    (Actor|DestroyActor)))

(event EventTick
  (params (DeltaSeconds :type Float%20%28single-precision%29))
  (bind _staticmesh (Variables|Default|GetStaticMesh))
  ;[1 1 1] Highlight
  (if (stale Custom|AddToInv _success)
    (Rendering|SetRenderCustomDepth _staticmesh false)
    (Rendering|SetCustomDepthStencilValue _staticmesh 0)))

(fn ConstructionScript)