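; Nail attachment pickup in the weapons set that the player can interact with to add one to their inventory.
; Interact passes the item struct to the player's InventoryComponent and destroys the actor if the add succeeds; a separate Destroy event also removes it.
; The Highlight component's overlap toggles custom depth and stencil on the mesh for an outline-style highlight.
; Tick clears that highlight once the item has been added.
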(event OnComponentBeginOverlap(Highlight)
  (params (OverlappedComponent :type Primitive%20Component%20Object%20Reference) (OtherActor :type Actor%20Object%20Reference) (OtherComp :type Primitive%20Component%20Object%20Reference) (OtherBodyIndex :type Integer) (bFromSweep :type Boolean) (SweepResult :type Hit%20Result%20Structure%20%28by%20ref%29))
  (bind _staticmesh (Variables|Default|GetStaticMesh))
  (Rendering|SetRenderCustomDepth _staticmesh true)
  (Rendering|SetCustomDepthStencilValue _staticmesh 2))

(event OnComponentEndOverlap(Highlight)
  (params (OverlappedComponent :type Primitive%20Component%20Object%20Reference) (OtherActor :type Actor%20Object%20Reference) (OtherComp :type Primitive%20Component%20Object%20Reference) (OtherBodyIndex :type Integer))
  (bind _staticmesh (Variables|Default|GetStaticMesh))
  (Rendering|SetRenderCustomDepth _staticmesh false)
  (Rendering|SetCustomDepthStencilValue _staticmesh 0))

(event Custom|Destroy
  (Actor|DestroyActor))

(event EventBeginPlay)

(event Collision|EventActorBeginOverlap
  (params (OtherActor :type Actor%20Object%20Reference)))

(event EventInteract
  (params (Interacter :type Actor%20Object%20Reference) (HasWeapon :type Boolean))
  (bind _success (Default|AddtoInventory (Actor|GetComponentbyClass (Game|GetPlayerCharacter 0) "/Game/InventorySystem/InventoryComponent.InventoryComponent_C") (Utilities|Struct|MakeSlotStruct (Variables|Default|Getstruct) 1)))
  (if _success
    (Actor|DestroyActor)))

(event EventTick
  (params (DeltaSeconds :type Float%20%28single-precision%29))
  (bind _staticmesh (Variables|Default|GetStaticMesh))
  (if (stale EventInteract _success)
    (Rendering|SetRenderCustomDepth _staticmesh false)
    (Rendering|SetCustomDepthStencilValue _staticmesh 0)))

(fn ConstructionScript)