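; Elevator doors Blueprint that slides two doors open when the player approaches and closes them when the player leaves.
; BeginPlay caches the player's ThirdPersonCharacter, and a Trigger volume checks overlaps against that reference.
; Overlap begin plays the DoorAnim timeline, which drives each door's relative X location from its own track; overlap end reverses the same timeline.
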(event OnComponentBeginOverlap(Trigger)
  (params (OverlappedComponent :type Primitive%20Component%20Object%20Reference) (OtherActor :type Actor%20Object%20Reference) (OtherComp :type Primitive%20Component%20Object%20Reference) (OtherBodyIndex :type Integer) (bFromSweep :type Boolean) (SweepResult :type Hit%20Result%20Structure%20%28by%20ref%29))
  (if (== OtherActor (Variables|Default|GetPlayerRef))
    (bind (_direction _door1open _door2open) (Timeline|DoorAnim Play)
      (:Update
        (Transformation|SetRelativeLocation (Variables|Default|GetDoor1) (Math|Vector|MakeVector _door1open 0.0 0.0) false false)
        (Transformation|SetRelativeLocation (Variables|Default|GetDoor2) (Math|Vector|MakeVector _door2open 0.0 0.0) false false)))))

(event OnComponentEndOverlap(Trigger)
  (params (OverlappedComponent :type Primitive%20Component%20Object%20Reference) (OtherActor :type Actor%20Object%20Reference) (OtherComp :type Primitive%20Component%20Object%20Reference) (OtherBodyIndex :type Integer))
  (if (== OtherActor (Variables|Default|GetPlayerRef))
    (bind (_direction _door1open _door2open) (Timeline|DoorAnim Reverse)
      (:Update
        (Transformation|SetRelativeLocation (Variables|Default|GetDoor1) (Math|Vector|MakeVector _door1open 0.0 0.0) false false)
        (Transformation|SetRelativeLocation (Variables|Default|GetDoor2) (Math|Vector|MakeVector _door2open 0.0 0.0) false false)))))

(event EventBeginPlay
  (bind _asthird_person_character (Utilities|Casting|CastToThirdPersonCharacter (Game|GetPlayerCharacter 0)))
  (Variables|Default|SetPlayerRef _asthird_person_character))

(fn ConstructionScript)