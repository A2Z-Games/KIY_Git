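; Player controller that creates the HUD widget at BeginPlay and handles inventory and interaction input.
; The Inventory input toggles the InventoryComponent's window, while Interact sphere-traces around the player character on one object type and sends InteractMessage to a hit actor implementing Interact_Interface.
; It also records a first and second selected inventory slot with their indices, and ResetClicks clears that selection.
; EmptySlot is an unimplemented stub.
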(event Custom|slectSlot
  (params (SelctedSlot :type Slot%20Structure%20NEW%20Structure) (SlotIndex :type Integer))
  ;[1 1 1] selects 2 slots
  (if (Variables|Default|GetslotOneSelected)
    (Variables|Default|SetSelectedSlot2 SelctedSlot)
    (Variables|Default|SetSelectedSlotIndex2 SlotIndex)
    (else
      (bind _output_get (Variables|Default|SetSelectedSlot SelctedSlot))
      (Variables|Default|SetSelectedSlotIndex SlotIndex)
      (Variables|Default|SetslotOneSelected true))))

(event EventBeginPlay
  ;[0 0.7874 1 1 56] UI
  ;;[1 1 1] CreateHUD
  (bind _returnvalue (UserInterface|CreateWidget "/Game/NewInventoryAndCraftimgSystems/InventoryUI/HUD.HUD_C"))
  (bind _output_get (Variables|Default|SetHUD%20Widget _returnvalue))
  (UserInterface|Viewport|AddtoViewport _output_get 0))

(event Input|ActionEvents|InputActionInventory
  (params (Key :type Key%20Structure :default "None"))
  ;[0 0.7874 1 1 56] UI
  ;;[1 1 1] Toggling inventory window by pressing Tab
  (:Pressed
    (Default|ToggleInventory (Variables|Default|GetInventoryComponent))))

(event Input|ActionEvents|InputActionInteract
  (params (Key :type Key%20Structure :default "None"))
  (bind _returnvalue (Game|GetPlayerCharacter 0))
  ;[1 1 1] interact interface logic
  (:Pressed
    (bind _outhit (Collision|SphereTraceForObjects (Transformation|GetWorldLocation (Variables|/Script/Engine.Actor|GetRootComponent _returnvalue)) (+ (Transformation|GetWorldLocation (Variables|/Script/Engine.Actor|GetRootComponent _returnvalue)) 3e+01) 1e+02 (Utilities|Array|MakeArray "ObjectTypeQuery8") false 0 "None"))
    (if (Utilities|DoesObjectImplementInterface (.hitactor _outhit) "/Game/InventorySystem/Interact_Interface.Interact_Interface_C")
      (Class|InteractInterface|Interact(Message) (.hitactor _outhit)))))

(fn ConstructionScript)

(fn ResetClicks
  (Variables|Default|SetSelectedSlot "")
  (Variables|Default|SetSelectedSlot2 "")
  (Variables|Default|SetslotOneSelected false))

(fn EmptySlot)