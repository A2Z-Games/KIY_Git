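; Enemy character Blueprint that takes weapon hits, dies into a ragdoll and makes melee attacks on the player.
; EnemyHit plays a reaction and sound, notifies the weapon of breakage and subtracts fixed Health, ignoring WeaponDmg.
; At zero Health it starts a death montage, enables mesh physics, disables capsule collision and sets Dead.
; MeleeAttack, if alive, plays a montage and messages the player pawn after a delay, without any range check.
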(event Custom|EnemyHit
  (params (PickedUpWeapon :type Actor%20Object%20Reference) (WeaponDmg :type Integer))
  (bind _mesh (Variables|Character|GetMesh))
  (Animation|PlayAnimMontage "/Game/Animations/EnemyAnimations/Standing_React_Small_From_Front_02_Montage.Standing_React_Small_From_Front_02_Montage" 1.5 "None")
  (Variables|Default|SetHealth (- (Variables|Default|GetHealth) 40))
  (Audio|PlaySoundatLocation "/Game/KIY/DEV/Tomer/172004__skinnysoundguy__creature-beast-retch.172004__skinnysoundguy__creature-beast-retch" (Transformation|GetWorldLocation (Variables|Collision|GetCapsuleComponent)) "0, 0, 0" 1.0 1.0 0.0 0 0 0)
  (Class|WeaponsInterface|Break(Message) PickedUpWeapon)
  (if (<= (Variables|Default|GetHealth) 0)
    (Animation|PlayAnimMontage "/Game/Animations/EnemyAnimations/Sword_And_Shield_Death_Montage.Sword_And_Shield_Death_Montage" 1.5 "None")
    (Collision|SetCollisionProfileName _mesh "Ragdoll" :!class /Script/Engine.PrimitiveComponent)
    (Physics|SetSimulatePhysics _mesh true)
    (Collision|SetCollisionEnabled (Variables|Collision|GetCapsuleComponent) "NoCollision")
    (Variables|Default|SetDead true)))

(event EventBeginPlay)

(event Collision|EventActorBeginOverlap
  (params (OtherActor :type Actor%20Object%20Reference)))

(event EventMeleeAttack
  (if (not (Variables|Default|GetDead))
    (Animation|Montage|PlayMontage (Variables|Character|GetMesh) "/Game/Animations/EnemyAnimations/hkjh.hkjh" 1.5
      (:then
        (Utilities|FlowControl|Delay 1.0)
        (Class|EnemytoPlayerAttackInterface|EnemyHitPlayer(Message) (Game|Player|GetPlayerPawn 0))))))

(fn ConstructionScript)